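; Player character with axis-driven movement and look, a HUD and a hitscan attack against enemies.
; BeginPlay adds the UMG_HUD widget to the viewport and sets starting life, maximum life and damage values.
; Movement follows the control rotation's forward and right vectors, while look axes feed controller yaw and pitch.
; Left click line-traces along the capsule's forward vector, not the view direction, with debug drawing, and damages any BP_Enemy hit.
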(event `Key|LeftMouseButton`
  (params (Key :type "Key Structure"))
  (bind _capsulecomponent (`self.CapsuleComponent`))
  (bind _returnvalue (`SceneComponent.K2_GetComponentLocation` _capsulecomponent))
  (:`Pressed`
    (bind _outhit (`KismetSystemLibrary.LineTraceSingle` :`Start` _returnvalue :`End` (+ (* (`SceneComponent.GetForwardVector` _capsulecomponent) 1000) _returnvalue) :`TraceChannel` "TraceTypeQuery1" :`DrawDebugType` "ForDuration"))
    (bind _asbp_enemy (cast `/Game/BluePrint/BP_Enemy` (`.HitActor` (`GameplayStatics.BreakHitResult` _outhit))))
    (`self.TakeDamage` _asbp_enemy (`self.Damage`))))

(event `self.ReceiveBeginPlay`
  (`parent.ReceiveBeginPlay`)
  (bind _returnvalue (`|CreateWidget` "/Game/UMG/UMG_HUD.UMG_HUD_C"))
  (`UserWidget.AddToViewport` _returnvalue 0)
  (set `self.LifeMax` 100)
  (set `self.Life` 80)
  (set `self.Damage` 10))

(event `InputAxis|Avant`
  (params (AxisValue :type "Float (single-precision)"))
  (`self.AddMovementInput` (`KismetMathLibrary.GetForwardVector` (`self.GetControlRotation`)) AxisValue))

(event `InputAxis|Droite`
  (params (AxisValue :type "Float (single-precision)"))
  (`self.AddMovementInput` (`KismetMathLibrary.GetRightVector` (`self.GetControlRotation`)) AxisValue))

(event `InputAxis|Tourner`
  (params (AxisValue :type "Float (single-precision)"))
  (`self.AddControllerYawInput` AxisValue))

(event `InputAxis|LookUp`
  (params (AxisValue :type "Float (single-precision)"))
  (`self.AddControllerPitchInput` AxisValue))

(fn `UserConstructionScript`
  (`parent.UserConstructionScript`))