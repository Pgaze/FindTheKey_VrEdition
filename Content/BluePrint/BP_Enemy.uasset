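; BP_Enemy is an enemy Blueprint that turns to face the player each frame.
; BeginPlay initializes its current and maximum life, though nothing in the file changes them afterward.
; Tick casts the player character to BP_Player and sets the capsule component's world rotation toward it with a look-at rotation, so the facing snaps without interpolation.
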(event `self.ReceiveBeginPlay`
  (`parent.ReceiveBeginPlay`)
  (set `self.LifeMax` 100)
  (set `self.Life` 100))

(event `self.ReceiveTick`
  (params (DeltaSeconds :type "Float (single-precision)"))
  (`parent.ReceiveTick` DeltaSeconds)
  (bind _asbp_player (cast `/Game/BluePrint/BP_Player` (`GameplayStatics.GetPlayerCharacter` 0)))
  (`SceneComponent.K2_SetWorldRotation` (`self.CapsuleComponent`) (`KismetMathLibrary.FindLookAtRotation` (`self.K2_GetActorLocation`) (`self.K2_GetActorLocation` _asbp_player)) false false))

(fn `UserConstructionScript`
  (`parent.UserConstructionScript`))